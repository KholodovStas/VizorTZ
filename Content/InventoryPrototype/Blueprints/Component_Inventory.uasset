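; Inventory component that holds a fixed number of item slots and toggles an inventory window on the player controller's HUD canvas, switching input mode.
; AddToInventory uses the Stack macro to find a partly filled slot of the same actor class for stackable items, otherwise writing to the first empty slot.
; AddToStack caps a slot at the stack size and recursively adds any overflow.
; AddToInventory always returns true, with no explicit full-inventory check.
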(event EventBeginPlay
  (CallFunction|PrepareInventory))

(fn ToggleInventory
  (bind _inventorywindow (Variables|Default|GetInventoryWindow)
    (:then
      (Widget|RemovefromParent _inventorywindow)
      (Variables|Default|SetInventoryWindow 0)
      (Input|SetInputModeGameOnly (Game|GetPlayerController 0)))
    (:else
      (bind _returnvalue (UserInterface|CreateWidget "/Game/InventoryPrototype/Widgets/WB_InventoryWindow.WB_InventoryWindow_C" 0 self))
      (Variables|Default|SetInventoryWindow _returnvalue)
      (bind _asbp_player_controller (Utilities|Casting|CastToBP_PlayerController (Game|GetPlayerController 0)))
      (bind _returnvalue_2 (Class|CanvasPanel|AddChildtoCanvas (Variables|/Game/InventoryPrototype/Widgets/HUD.HUD_C|GetCanvasPanel_Hud (Variables|/Game/InventoryPrototype/Blueprints/BP_PlayerController.BP_PlayerController_C|GetHUD _asbp_player_controller)) (Variables|Default|GetInventoryWindow)))
      (Class|CanvasPanelSlot|SetAutoSize _returnvalue_2 true)
      (Class|CanvasPanelSlot|SetAlignment _returnvalue_2 "(X=-0.500000,Y=-0.500000)")
      (Input|SetInputModeUIOnly (Game|GetPlayerController 0) (Variables|Default|GetInventoryWindow) "LockAlways"))))

(fn AddtoInventory
  (params (ContentAdd :type Structure%20Slot%20Structure))
  (if (.isstackable (.itemstructure ContentAdd))
    (bind _stackindex (Utilities|Stack ContentAdd)
      (:True
        (CallFunction|AddtoStack ContentAdd _stackindex))
      (:False
        (CallFunction|CreateStack ContentAdd :!label _label)))
    (else
      (goto _label)))
  (return true))

(fn PrepareInventory
  (Utilities|Array|Resize (Variables|Default|GetInventory) (Variables|Default|GetNumberOfSlots)))

(fn CreateStack
  (params (Content :type Structure%20Slot%20Structure))
  (bind _inventory (Variables|Default|GetInventory))
  (Utilities|Array|SetArrayElem _inventory (Utilities|Array|FindItem _inventory (Utilities|Struct|MakeStructure_Slot "(Name_2_197EE7184189423A34FE329208298D4F=\"\",IsStackable_9_F31318A94A875D33ADEA3BA92CB62A59=False,Image_13_2AB1517B46E3222337180AB80F388B8A=None,Description_15_EC6ECAC749DCE45DDDBDB1A80B07B63A=\"\",StackSize_18_C5EF8F43432C837B0DEE96AC9A1370CA=0,ActorClass_23_4B236B8A4E9CFC6C0D892091B2F2A5A3=None)")) Content))

(fn AddtoStack
  (params (SlotStructure :type Structure%20Slot%20Structure) (SlotIndex :type Integer))
  (bind _inventory (Variables|Default|GetInventory))
  (bind _inventory_2 (Variables|Default|GetInventory))
  (bind _stacksize (Utilities|Struct|BreakStructure_Item (.itemstructure SlotStructure)))
  (bind _output (Utilities|Array|Get(acopy) _inventory SlotIndex))
  (bind _output_2 (Utilities|Array|Get(acopy) _inventory_2 SlotIndex))
  (bind _output_get (LocalVariables|SetQuantity (.quantity _output)))
  (if (> (+ _output_get (.Quantity (Utilities|Struct|BreakStructure_Slot SlotStructure))) (.stacksize (.itemstructure _output)))
    (Utilities|Array|SetArrayElem (Variables|Default|GetInventory) SlotIndex (Utilities|Struct|MakeStructure_Slot (.itemstructure SlotStructure) _stacksize))
    (CallFunction|AddtoInventory (Utilities|Struct|MakeStructure_Slot (.itemstructure SlotStructure) (- (.quantity SlotStructure) (- _stacksize (LocalVariables|GetQuantity)))))
    (else
      (Utilities|Array|SetArrayElem _inventory_2 SlotIndex (Utilities|Struct|MakeStructure_Slot (.itemstructure _output_2) (+ (.quantity _output_2) (.quantity SlotStructure))))))
  (return))