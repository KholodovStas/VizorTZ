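; BP_Item is a world pickup that adds one of its item to the interacting actor's Component_Inventory, then destroys itself.
; CheckForCompleteness scans that inventory for an empty slot or unfilled matching stack, counting occupied slots against a hardcoded limit.
; A sphere overlap by ThirdPersonCharacter uses the same check to show either a press-E prompt or an inventory-full message on a widget, hidden when overlap ends.
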(event OnComponentBeginOverlap(Sphere)
  (params (OverlappedComponent :type Primitive%20Component%20Object%20Reference) (OtherActor :type Actor%20Object%20Reference) (OtherComp :type Primitive%20Component%20Object%20Reference) (OtherBodyIndex :type Integer) (bFromSweep :type Boolean) (SweepResult :type Hit%20Result%20Structure%20%28by%20ref%29))
  (bind _asthird_person_character (Utilities|Casting|CastToThirdPersonCharacter OtherActor))
  (bind _isfull (CallFunction|CheckforCompleteness _asthird_person_character))
  (if _isfull
    (bind _aswb_item_text (Utilities|Casting|CastToWB_ItemText (UserInterface|GetUserWidgetObject (Variables|Default|GetWidget))))
    (Variables|/Game/InventoryPrototype/Widgets/WB_ItemText.WB_ItemText_C|SetText _aswb_item_text "Press \"E\"")
    (else
      (bind _aswb_item_text_2 (Utilities|Casting|CastToWB_ItemText (UserInterface|GetUserWidgetObject (Variables|Default|GetWidget))))
      (Variables|/Game/InventoryPrototype/Widgets/WB_ItemText.WB_ItemText_C|SetText _aswb_item_text_2 "Inventory is full")))
  (Rendering|SetVisibility (Variables|Default|GetWidget) true false))

(event OnComponentEndOverlap(Sphere)
  (params (OverlappedComponent :type Primitive%20Component%20Object%20Reference) (OtherActor :type Actor%20Object%20Reference) (OtherComp :type Primitive%20Component%20Object%20Reference) (OtherBodyIndex :type Integer))
  (Utilities|Casting|CastToThirdPersonCharacter OtherActor)
  (Rendering|SetVisibility (Variables|Default|GetWidget) false false))

(event EventInteract
  (params (Actor :type Actor%20Object%20Reference))
  (bind _isfull (CallFunction|CheckforCompleteness Actor))
  (if _isfull
    (Default|AddtoInventory (Actor|GetComponentbyClass Actor "/Game/InventoryPrototype/Blueprints/Component_Inventory.Component_Inventory_C") (Utilities|Struct|MakeStructure_Slot (Variables|Default|GetItemStructure) 1))
    (Actor|DestroyActor)))

(fn ConstructionScript)

(fn CheckforCompleteness
  (params (ComponentInventory :type Actor%20Object%20Reference))
  (bind _itemstructure (Variables|Default|GetItemStructure))
  (bind _array_element (Utilities|Array|ForEachLoopwithBreak (Variables|/Game/InventoryPrototype/Blueprints/Component_Inventory.Component_Inventory_C|GetInventory (Actor|GetComponentbyClass ComponentInventory "/Game/InventoryPrototype/Blueprints/Component_Inventory.Component_Inventory_C")) :!label _label)
    (:LoopBody
      (if (>= (.quantity _array_element) 1)
        (if (Utilities|Enum|Equal(Enum) (.name (.itemstructure _array_element)) (.name _itemstructure))
          (if (.isstackable _itemstructure)
            (if (< (.quantity _array_element) (.stacksize _itemstructure))
              (goto _label Break)
              (else
                (LocalVariables|SetSizeInventory (+ (LocalVariables|GetSizeInventory) 1))))
            (else
              (LocalVariables|SetSizeInventory (+ (LocalVariables|GetSizeInventory) 1) :!label _label_2)))
          (else
            (goto _label_2)))
        (else
          (goto _label Break))))
    (:Completed
      (return (<= (LocalVariables|GetSizeInventory) 15)))))